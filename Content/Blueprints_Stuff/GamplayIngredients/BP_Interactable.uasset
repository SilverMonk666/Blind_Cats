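; BP_Interactable is a base-style interactable that registers itself with BP_MainCharacter_ while the character is inside its Box.
; Begin overlap sets the character's CanInteractWith flag and BPInteractable reference, gated by a DoOnce.
; End overlap by that character clears both and resets the gate.
; InteractWith takes a player reference but is an empty stub here, so this Blueprint defines no interaction behavior.
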(event OnComponentBeginOverlap(Box)
  (params (OverlappedComponent :type Primitive%20Component%20Object%20Reference) (OtherActor :type Actor%20Object%20Reference) (OtherComp :type Primitive%20Component%20Object%20Reference) (OtherBodyIndex :type Integer) (bFromSweep :type Boolean) (SweepResult :type Hit%20Result%20Structure%20%28by%20ref%29))
  (bind _asbp_main_character_ (Utilities|Casting|CastToBP_MainCharacter_ OtherActor))
  (Utilities|FlowControl|DoOnce false
    (:Completed
      (bind _output_get (Variables|Default|SetAs%20BP%20Main%20Character _asbp_main_character_))
      (Variables|/Game/Blueprints_Stuff/Character/BP_MainCharacter_.BP_MainCharacter__C|SetCanInteractWith? _output_get true)
      (Variables|/Game/Blueprints_Stuff/Character/BP_MainCharacter_.BP_MainCharacter__C|SetBP_Interactable _output_get self))))

(event OnComponentEndOverlap(Box)
  (params (OverlappedComponent :type Primitive%20Component%20Object%20Reference) (OtherActor :type Actor%20Object%20Reference) (OtherComp :type Primitive%20Component%20Object%20Reference) (OtherBodyIndex :type Integer))
  (bind _as_bp_main_character (Variables|Default|GetAs%20BP%20Main%20Character))
  (if (== OtherActor _as_bp_main_character)
    (Variables|/Game/Blueprints_Stuff/Character/BP_MainCharacter_.BP_MainCharacter__C|SetBP_Interactable _as_bp_main_character 0)
    (Variables|/Game/Blueprints_Stuff/Character/BP_MainCharacter_.BP_MainCharacter__C|SetCanInteractWith? _as_bp_main_character false)
    (CallFunction|Reset)))

(event Custom|Reset
  (Utilities|FlowControl|DoOnce false) ; enters at Reset
)

(fn ConstructionScript)

(fn Interactwith
  (params (PlayerRef :type BP%20Main%20Character%20Object%20Reference)))